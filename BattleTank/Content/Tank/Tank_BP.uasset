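; Player-controllable tank Blueprint that drives, aims and fires.
; On BeginPlay it hands both tracks to TankMovement, the barrel and turret to TankAiming, and itself to a HealthBar widget.
; Drive and turn axes send intents to TankMovement, and Shoot calls Fire on TankAiming.
; Aim axes rotate the azimuth gimbal and spring arm separately, scaled by delta time, rather than moving the turret directly.
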(event `self.ReceiveBeginPlay`
  (`TankMovementComponent.Initialise` (`self.TankMovement`) (`self.LeftTrack`) (`self.RightTrack`))
  (`TankAimingComponent.Initialise` (`self.TankAiming`) (`self.Barrel`) (`self.TankTurret`))
  (`self.InitialiseHealthBarWidget`))

(event `InputAxis|AimAzimuth`
  (params (AxisValue :type "Float (single-precision)"))
  ;[1 1 1] Ballistic input bindings
  (`SceneComponent.K2_AddLocalRotation` (`self.Azimuth Gimbul`) (`KismetMathLibrary.MakeRotator` 0.0 0.0 (* AxisValue (`GameplayStatics.GetWorldDeltaSeconds`) 100.0)) false false))

(event `InputAxis|LineMovement`
  (params (AxisValue :type "Float (single-precision)"))
  ;[1 1 1] Movement Input Binding
  (`TankMovementComponent.IntendMoveForward` (`self.TankMovement`) AxisValue))

(event `InputAxis|TurnRight`
  (params (AxisValue :type "Float (single-precision)"))
  ;[1 1 1] Movement Input Binding
  (`TankMovementComponent.IntendTurnRight` (`self.TankMovement`) AxisValue))

(event `InputAxis|AimElevation`
  (params (AxisValue :type "Float (single-precision)"))
  ;[1 1 1] Ballistic input bindings
  (`SceneComponent.K2_AddLocalRotation` (`self.SpringArm`) (`KismetMathLibrary.MakeRotator` 0.0 (* (`GameplayStatics.GetWorldDeltaSeconds`) AxisValue 100.0)) false false))

(event `InputAction|Shoot`
  (params (Key :type "Key Structure"))
  ;[1 1 1] Ballistic input bindings
  (:`Pressed`
    (`TankAimingComponent.Fire` (`self.TankAiming`))))

(fn `InitialiseHealthBarWidget`
  (bind _ashealth_bar (cast `/Game/Blueprints/HealthBar` (`WidgetComponent.GetUserWidgetObject` (`self.Widget`))))
  (set `/Game/Blueprints/HealthBar.Tank` self _ashealth_bar))

(fn `UserConstructionScript`)